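; Level exit door that, once opened, walks the overlapping ALS player character through it and loads the next level.
; Open sets IsOpen and plays a timeline meant to swing the door's yaw.
; Trigger overlap takes control from the player, runs a delay-sequenced turn, position and walk-forward cutscene, then calls NextLevel on ALS_GameMode_SP.
; The construction script gives the plane a dynamic material with a black top color.
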(event OnComponentBeginOverlap(Trigger)
  (params (OverlappedComponent :type Primitive%20Component%20Object%20Reference) (OtherActor :type Actor%20Object%20Reference) (OtherComp :type Primitive%20Component%20Object%20Reference) (OtherBodyIndex :type Integer) (bFromSweep :type Boolean) (SweepResult :type Hit%20Result%20Structure%20%28by%20ref%29))
  (bind _asals_anim_man_character_bp (Utilities|Casting|CastToALS_AnimMan_CharacterBP OtherActor))
  (if (Variables|Default|GetisOpen)
    (Variables|Default|SetPlayerCharacter _asals_anim_man_character_bp)
    (CallFunction|RemoveControl)
    (if (CallFunction|PlayerFacingOutorin)
      (bind _delay (CallFunction|TurnRight))
      (Utilities|FlowControl|Delay _delay))
    (CallFunction|GetinPosition)
    (if (< (Math|Float|Absolute(Float) (CallFunction|PlayerYaw)) 1.0)
      (bind _delay_2 (CallFunction|TurnLeft))
      (Utilities|FlowControl|Delay _delay_2)
      (else
        (bind _delay_3 (CallFunction|TurnRight))
        (Utilities|FlowControl|Delay _delay_3)))
    (bind _delay_4 (CallFunction|WalkForward 2.0))
    (Utilities|FlowControl|Delay _delay_4)
    (bind _asals_game_mode_sp (Utilities|Casting|CastToALS_GameMode_SP (Game|GetGameMode)))
    (Default|NextLevel _asals_game_mode_sp (Variables|Default|GetNextLevel))))

(event EventBeginPlay)

(event Collision|EventActorBeginOverlap
  (params (OtherActor :type Actor%20Object%20Reference)))

(event EventTick
  (params (DeltaSeconds :type Float%20%28single-precision%29)))

(fn ConstructionScript
  (bind _returnvalue (Rendering|Material|CreateDynamicMaterialInstance "/Game/AdvancedLocomotionV4/Environment/Materials/M_Object.M_Object" "None" "None" :!class /Script/Engine.KismetMaterialLibrary))
  (Rendering|Material|SetVectorParameterValue _returnvalue "TopColor_1" "(R=0.000000,G=0.000000,B=0.000000,A=1.000000)" :!class /Script/Engine.MaterialInstanceDynamic)
  (Rendering|Material|SetMaterial (Variables|Default|GetPlane) 0 _returnvalue))

(fn Open
  (Variables|Default|SetisOpen true)
  (Audio|Components|Audio|Play (Variables|Default|GetTimeline)))