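; Generated dynamic mesh actor that procedurally builds a parametric wall segment with a window opening.
; On rebuild, Geometry Script primitives form a square or rounded wall, then booleans add border and trim, cut the opening, and insert glass.
; Optional plane cuts, a curved revolved extension with trim, mirroring and polygroup bevels shape the result.
; Per-part material IDs map to wall, border, glass and trim materials.
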(event EventBeginPlay
  (|CallParentFunction) ; This node is disabled and will not be called.\nDrag off pins to build functionality.
)

(event EventTick
  (params (DeltaSeconds :type Float%20%28single-precision%29))
  (|CallParentFunction DeltaSeconds) ; This node is disabled and will not be called.\nDrag off pins to build functionality.
)

(event Events|EventOnRebuildGeneratedMesh
  (params (TargetMesh :type Dynamic%20Mesh%20Object%20Reference))
  (bind (_location _axis) (|GetLocationAndAxis))
  (bind _wallcornerradius (Variables|Settings|Wall|GetWallCornerRadius))
  (bind _wallheight (Variables|Settings|Wall|GetWallHeight))
  (Variables|Default|SetDynamicMEsh TargetMesh)
  (switch Utilities|FlowControl|Switch|SwitchonEnum_WindowType (Variables|Settings|Wall|GetWallCorner)
    (:NewEnumerator0
      ;[1 1 1] Wall
      (bind _returnvalue (Class|GeometryScriptLibraryMeshPrimitiveFunctions|AppendBox :TargetMesh (Variables|Default|GetDynamicMEsh) :DimensionX (Variables|Settings|Wall|GetWallWidth) :DimensionY (Variables|Settings|Wall|GetWallThickness) :DimensionZ (Variables|Settings|Wall|GetWallHeight) :StepsX 1 :StepsY 1 :StepsZ 1 :Debug 0))
      (Variables|Default|SetDynamicMEsh _returnvalue))
    (:NewEnumerator1
      (bind _returnvalue_2 (Class|GeometryScriptLibraryMeshPrimitiveFunctions|AppendRoundRectangleCompatibility50 :TargetMesh (Variables|Default|GetDynamicMEsh) :Transform (Math|Transform|MakeTransform (Math|Vector|MakeVector 0.0 (* (/ (Variables|Settings|Wall|GetWallThickness) 2.0) -1.0) (/ _wallheight 2.0)) "0,0.000000,90.000000" "1.000000,1.000000,1.000000") :DimensionX (|((Axis*2)-(CR*4)) (Variables|Settings|Wall|GetWallWidth) _wallcornerradius) :DimensionY (|((Axis*2)-(CR*4)) _wallheight _wallcornerradius) :CornerRadius _wallcornerradius :StepsRound (Variables|Settings|Wall|GetWallStepsRound) :Debug 0))
      (bind _returnvalue_3 (Class|GeometryScriptLibraryMeshModelingFunctions|ApplyMeshExtrudeCompatibility5p0 _returnvalue_2 (Utilities|Struct|MakeGeometryScriptMeshExtrudeOptions (Variables|Settings|Wall|GetWallThickness) "0.000000,1.000000,0.000000" 1.0 true) 0))
      (Variables|Default|SetDynamicMEsh _returnvalue_3)))
  (if (and (Variables|Settings|Bevel|GetbBevelWall) (not (Variables|Settings|Bevel|GetbBevelCombine)))
    ;[1 1 1] Wall Only Bevel
    (bind _target_mesh (CallFunction|FnBevel (Variables|Default|GetDynamicMEsh) (Variables|Settings|Bevel|GetBevelDistanceWall)))
    (Variables|Default|SetDynamicMEsh _target_mesh))
  ;[1 1 1] Window Border + Trim + Window + Glass + Side Cutters
  (Utilities|McWindowBorder) ; Window Border
  (Utilities|McTrim ; Trim
    (:OutputPin
      (Utilities|McWindowCut) ; Window Cut
      (Utilities|McGlassPiece ; Glass Piece
        (:Output%20Pin
          ;;[1 1 1] Side Cutters
          (Utilities|McGroundCut
            (:OutputPin
              (Utilities|McTopCut
                (:OutputPin
                  (Utilities|McLeftCut
                    (:OutputPin
                      (Utilities|McRightCut
                        (:OutputPin
                          (if (Variables|Settings|ExtendWalls|GetbExtendWall)
                            ;[1 1 1] Wall Exentsion
                            (CallFunction|FnCreateExtend) ; Wall Extension
                            (if (and (Variables|Settings|Trim|GetbVertical) (Variables|Settings|Trim|GetbHasTrim))
                              ;[1 1 1] Add Trim to Wall Extension (Horizontal or Vertical Based on Wall Extension Design
                              (switch Utilities|FlowControl|Switch|SwitchonEnum_RailingConstructionType (Variables|Settings|Trim|GetTrimType)
                                (:NewEnumerator0
                                  (CallFunction|FnCreateExtendTrim "NewEnumerator0"))
                                (:NewEnumerator1
                                  (CallFunction|FnCreateExtendTrim "NewEnumerator1"))
                                (:NewEnumerator2
                                  (CallFunction|FnCreateExtendTrim "NewEnumerator1")
                                  (CallFunction|FnCreateExtendTrim "NewEnumerator0")))))
                          (DynamicMeshActor|ReleaseAllComputeMeshes)
                          (bind _returnvalue_4 (Class|GeometryScriptLibraryMeshNormalsFunctions|ComputeSplitNormals :TargetMesh (Variables|Default|GetDynamicMEsh) :SplitOptions (Utilities|Struct|MakeGeometryScriptSplitNormalsOptions true 25.0 false "(bDefaultLayer=True,ExtendedLayerIndex=0)") :Debug 0))
                          (Variables|Default|SetDynamicMEsh _returnvalue_4)
                          ;[1 1 1] Mirroring with Custom Options
                          (if (Variables|Settings|Mirror|GetbMirror)
                            (bind _returnvalue_5 (Class|GeometryScriptLibraryMeshBooleanFunctions|ApplyMeshMirror (Variables|Default|GetDynamicMEsh) (Math|Transform|MakeTransform _location _axis "1.000000,1.000000,1.000000") (Utilities|Struct|MakeGeometryScriptMeshMirrorOptions true true true) 0))
                            (Variables|Default|SetDynamicMEsh _returnvalue_5))
                          (if (Variables|Settings|Cutter|GetbCustomCutter)
                            ;[1 1 1] Custom Cutter
                            (Class|GeometryScriptLibraryMeshBooleanFunctions|ApplyMeshPlaneCut (Variables|Default|GetDynamicMEsh) (Math|Transform|MakeTransform (Variables|Settings|Cutter|GetCustomCutter) (Variables|Settings|Cutter|GetCustomCutterRotation) "1.000000,1.000000,1.000000") (Utilities|Struct|MakeGeometryScriptMeshPlaneCutOptions true true false 1.0) 0))
                          (if (Variables|Settings|Bevel|GetbBevelCombine)
                            ;[1 1 1] Bevel the whole thing
                            (bind _target_mesh_2 (CallFunction|FnBevel (Variables|Default|GetDynamicMEsh) (Variables|Settings|Bevel|GetBevelDistanceCombine)))
                            (Variables|Default|SetDynamicMEsh _target_mesh_2))
                          (CallFunction|CleanDegenerateTris (Variables|Default|GetDynamicMEsh) 0.0005 false true)
                          ;[1 1 1] Apply Materials
                          (Class|DynamicMeshComponent|ConfigureMaterialSet (Variables|Default|GetDynamicMeshComponent) (Utilities|Array|MakeArray (Variables|Settings|Wall|GetMaterialWall) (Variables|Settings|Opening|GetMaterialOpeningBorder) (Variables|Settings|Glass|GetMaterialGlass) (Variables|Settings|Trim|GetMaterialTrim))))))))))))))))

(event EventClearMaterials
  (bind (_location _axis) (|GetLocationAndAxis))
  (bind _wallcornerradius (Variables|Settings|Wall|GetWallCornerRadius))
  (bind _wallheight (Variables|Settings|Wall|GetWallHeight))
  ;[1 1 1] Clear Materials
  (Variables|Settings|Wall|SetMaterialWall 0)
  (Variables|Settings|Opening|SetMaterialOpeningBorder 0)
  (Variables|Settings|Glass|SetMaterialGlass 0)
  (Variables|Settings|Trim|SetMaterialTrim 0)
  (Variables|Default|SetDynamicMEsh (stale Events|EventOnRebuildGeneratedMesh TargetMesh))
  (switch Utilities|FlowControl|Switch|SwitchonEnum_WindowType (Variables|Settings|Wall|GetWallCorner)
    (:NewEnumerator0
      ;[1 1 1] Wall
      (bind _returnvalue (Class|GeometryScriptLibraryMeshPrimitiveFunctions|AppendBox :TargetMesh (Variables|Default|GetDynamicMEsh) :DimensionX (Variables|Settings|Wall|GetWallWidth) :DimensionY (Variables|Settings|Wall|GetWallThickness) :DimensionZ (Variables|Settings|Wall|GetWallHeight) :StepsX 1 :StepsY 1 :StepsZ 1 :Debug 0))
      (Variables|Default|SetDynamicMEsh _returnvalue))
    (:NewEnumerator1
      (bind _returnvalue_2 (Class|GeometryScriptLibraryMeshPrimitiveFunctions|AppendRoundRectangleCompatibility50 :TargetMesh (Variables|Default|GetDynamicMEsh) :Transform (Math|Transform|MakeTransform (Math|Vector|MakeVector 0.0 (* (/ (Variables|Settings|Wall|GetWallThickness) 2.0) -1.0) (/ _wallheight 2.0)) "0,0.000000,90.000000" "1.000000,1.000000,1.000000") :DimensionX (|((Axis*2)-(CR*4)) (Variables|Settings|Wall|GetWallWidth) _wallcornerradius) :DimensionY (|((Axis*2)-(CR*4)) _wallheight _wallcornerradius) :CornerRadius _wallcornerradius :StepsRound (Variables|Settings|Wall|GetWallStepsRound) :Debug 0))
      (bind _returnvalue_3 (Class|GeometryScriptLibraryMeshModelingFunctions|ApplyMeshExtrudeCompatibility5p0 _returnvalue_2 (Utilities|Struct|MakeGeometryScriptMeshExtrudeOptions (Variables|Settings|Wall|GetWallThickness) "0.000000,1.000000,0.000000" 1.0 true) 0))
      (Variables|Default|SetDynamicMEsh _returnvalue_3)))
  (if (and (Variables|Settings|Bevel|GetbBevelWall) (not (Variables|Settings|Bevel|GetbBevelCombine)))
    ;[1 1 1] Wall Only Bevel
    (bind _target_mesh (CallFunction|FnBevel (Variables|Default|GetDynamicMEsh) (Variables|Settings|Bevel|GetBevelDistanceWall)))
    (Variables|Default|SetDynamicMEsh _target_mesh))
  ;[1 1 1] Window Border + Trim + Window + Glass + Side Cutters
  (Utilities|McWindowBorder) ; Window Border
  (Utilities|McTrim ; Trim
    (:OutputPin
      (Utilities|McWindowCut) ; Window Cut
      (Utilities|McGlassPiece ; Glass Piece
        (:Output%20Pin
          ;;[1 1 1] Side Cutters
          (Utilities|McGroundCut
            (:OutputPin
              (Utilities|McTopCut
                (:OutputPin
                  (Utilities|McLeftCut
                    (:OutputPin
                      (Utilities|McRightCut
                        (:OutputPin
                          (if (Variables|Settings|ExtendWalls|GetbExtendWall)
                            ;[1 1 1] Wall Exentsion
                            (CallFunction|FnCreateExtend) ; Wall Extension
                            (if (and (Variables|Settings|Trim|GetbVertical) (Variables|Settings|Trim|GetbHasTrim))
                              ;[1 1 1] Add Trim to Wall Extension (Horizontal or Vertical Based on Wall Extension Design
                              (switch Utilities|FlowControl|Switch|SwitchonEnum_RailingConstructionType (Variables|Settings|Trim|GetTrimType)
                                (:NewEnumerator0
                                  (CallFunction|FnCreateExtendTrim "NewEnumerator0"))
                                (:NewEnumerator1
                                  (CallFunction|FnCreateExtendTrim "NewEnumerator1"))
                                (:NewEnumerator2
                                  (CallFunction|FnCreateExtendTrim "NewEnumerator1")
                                  (CallFunction|FnCreateExtendTrim "NewEnumerator0")))))
                          (DynamicMeshActor|ReleaseAllComputeMeshes)
                          (bind _returnvalue_4 (Class|GeometryScriptLibraryMeshNormalsFunctions|ComputeSplitNormals :TargetMesh (Variables|Default|GetDynamicMEsh) :SplitOptions (Utilities|Struct|MakeGeometryScriptSplitNormalsOptions true 25.0 false "(bDefaultLayer=True,ExtendedLayerIndex=0)") :Debug 0))
                          (Variables|Default|SetDynamicMEsh _returnvalue_4)
                          ;[1 1 1] Mirroring with Custom Options
                          (if (Variables|Settings|Mirror|GetbMirror)
                            (bind _returnvalue_5 (Class|GeometryScriptLibraryMeshBooleanFunctions|ApplyMeshMirror (Variables|Default|GetDynamicMEsh) (Math|Transform|MakeTransform _location _axis "1.000000,1.000000,1.000000") (Utilities|Struct|MakeGeometryScriptMeshMirrorOptions true true true) 0))
                            (Variables|Default|SetDynamicMEsh _returnvalue_5))
                          (if (Variables|Settings|Cutter|GetbCustomCutter)
                            ;[1 1 1] Custom Cutter
                            (Class|GeometryScriptLibraryMeshBooleanFunctions|ApplyMeshPlaneCut (Variables|Default|GetDynamicMEsh) (Math|Transform|MakeTransform (Variables|Settings|Cutter|GetCustomCutter) (Variables|Settings|Cutter|GetCustomCutterRotation) "1.000000,1.000000,1.000000") (Utilities|Struct|MakeGeometryScriptMeshPlaneCutOptions true true false 1.0) 0))
                          (if (Variables|Settings|Bevel|GetbBevelCombine)
                            ;[1 1 1] Bevel the whole thing
                            (bind _target_mesh_2 (CallFunction|FnBevel (Variables|Default|GetDynamicMEsh) (Variables|Settings|Bevel|GetBevelDistanceCombine)))
                            (Variables|Default|SetDynamicMEsh _target_mesh_2))
                          (CallFunction|CleanDegenerateTris (Variables|Default|GetDynamicMEsh) 0.0005 false true)
                          ;[1 1 1] Apply Materials
                          (Class|DynamicMeshComponent|ConfigureMaterialSet (Variables|Default|GetDynamicMeshComponent) (Utilities|Array|MakeArray (Variables|Settings|Wall|GetMaterialWall) (Variables|Settings|Opening|GetMaterialOpeningBorder) (Variables|Settings|Glass|GetMaterialGlass) (Variables|Settings|Trim|GetMaterialTrim))))))))))))))))

(fn ConstructionScript
  (|CallParentFunction))

(fn FnCreateTrim
  (params (Index :type Enum_RailingConstructionType%20Enum :default "NewEnumerator0"))
  (bind _bvertical (Variables|Settings|Trim|GetbVertical))
  (bind _bvertical_2 (Variables|Settings|Trim|GetbVertical))
  (bind _wallwidth (Variables|Settings|Wall|GetWallWidth))
  (bind _wallheight (Variables|Settings|Wall|GetWallHeight))
  (bind _returnvalue (/ _wallwidth 2.0))
  (bind _returnvalue_2 (DynamicMeshActor|AllocateComputeMesh))
  (bind _returnvalue_3 (Class|GeometryScriptLibraryMeshPrimitiveFunctions|AppendBox :TargetMesh _returnvalue_2 :Transform (Math|Transform|MakeTransform (Math|Vector|MakeVector 0.0 0.0 (Math|Float|SelectFloat 0.0 (Utilities|Select :Index Index :NewEnumerator0 0.0 :NewEnumerator1 (- _wallheight (Variables|Settings|Trim|GetTrimHeight)) :NewEnumerator2 0.0) _bvertical)) (Math|Rotator|MakeRotator 0.0 0.0 0.0) "1.000000,1.000000,1.000000") :DimensionX (Math|Float|SelectFloat (* _wallheight 2.0) (Variables|Settings|Wall|GetWallWidth) _bvertical) :DimensionY (+ (Variables|Settings|Wall|GetWallThickness) (Variables|Settings|Trim|GetTrimThickness)) :DimensionZ (Variables|Settings|Trim|GetTrimHeight) :Debug 0))
  (bind _returnvalue_4 (GeometryScript|Materials|RemapMaterialIDs _returnvalue_3 0 3 0))
  (bind _returnvalue_5 (GeometryScript|Booleans|ApplyMeshBoolean :TargetMesh (Variables|Default|GetDynamicMEsh) :ToolMesh _returnvalue_4 :ToolTransform (Math|Transform|MakeTransform (Math|Vector|MakeVector (Math|Float|SelectFloat (Utilities|Select :Index Index :NewEnumerator0 _returnvalue :NewEnumerator1 (+ (* _returnvalue -1.0) (Variables|Settings|Trim|GetTrimHeight)) :NewEnumerator2 0.0) 0.0 _bvertical_2) 0.0 0.0) (Math|Rotator|MakeRotator 0.0 (Math|Float|SelectFloat 9e+01 0.0 _bvertical_2) 0.0) "1.000000,1.000000,1.000000") :Operation "Union" :Debug 0))
  (Variables|Default|SetDynamicMEsh _returnvalue_5)
  (return))

(fn FnCreateExtend
  (bind _radius (Variables|Settings|ExtendWalls|GetRadius))
  (bind _wallthickness (Variables|Settings|Wall|GetWallThickness))
  (bind _wallwidth (Variables|Settings|Wall|GetWallWidth))
  (bind _wallthickness_2 (Variables|Settings|Wall|GetWallThickness))
  (bind _returnvalue (DynamicMeshActor|AllocateComputeMesh))
  (bind _returnvalue_2 (Class|GeometryScriptLibraryMeshPrimitiveFunctions|AppendRevolvePolygon :TargetMesh _returnvalue :Transform (Math|Transform|MakeTransform (Math|Vector|MakeVector (/ _wallwidth 2.0) (+ (Variables|Settings|ExtendWalls|GetRadius) (/ _wallthickness_2 2.0)) (Variables|Settings|Wall|GetWallHeight)) "0,90.000000,90.000000" "1.000000,1.000000,1.000000") :PolygonVertices (Utilities|Array|MakeArray (Math|Vector2D|MakeVector2D 0.0 0.0) (Math|Vector2D|MakeVector2D _wallthickness_2 0.0) (Math|Vector2D|MakeVector2D _wallthickness_2 _wallwidth) (Math|Vector2D|MakeVector2D 0.0 _wallwidth)) :RevolveOptions (Utilities|Struct|MakeGeometryScriptRevolveOptions 9e+01 -1.8e+02 false false 3e+01 false true) :Radius (Variables|Settings|ExtendWalls|GetRadius) :Debug 0))
  (bind _returnvalue_3 (GeometryScript|Booleans|ApplyMeshBoolean :TargetMesh (Variables|Default|GetDynamicMEsh) :ToolMesh _returnvalue_2 :Operation "Union" :Debug 0))
  (bind _returnvalue_4 (DynamicMeshActor|AllocateComputeMesh))
  (bind _returnvalue_5 (Class|GeometryScriptLibraryMeshPrimitiveFunctions|AppendBox :TargetMesh _returnvalue_4 :DimensionX (Variables|Settings|Wall|GetWallWidth) :DimensionY (Variables|Settings|Wall|GetWallThickness) :DimensionZ (Variables|Settings|ExtendWalls|GetExtensionLenght) :Debug 0))
  (bind _returnvalue_6 (GeometryScript|Booleans|ApplyMeshBoolean :TargetMesh _returnvalue_3 :ToolMesh _returnvalue_5 :ToolTransform (Math|Transform|MakeTransform (Math|Vector|MakeVector 0.0 (|((Thick/2)+Rad) _wallthickness _radius) (|(((Thick/2)+Height)+Rad) _wallthickness (Variables|Settings|Wall|GetWallHeight) _radius)) "0, 0,90.000000" "1.000000,1.000000,1.000000") :Operation "Union" :Debug 0))
  (Variables|Default|SetDynamicMEsh _returnvalue_6)
  (return))

(fn FnCreateExtendTrim
  (params (Type :type Enum_RailingConstructionType%20Enum :default "NewEnumerator1"))
  (bind _trimheight (Variables|Settings|Trim|GetTrimHeight))
  (bind _trimthickness (Variables|Settings|Trim|GetTrimThickness))
  (bind _radius (Variables|Settings|ExtendWalls|GetRadius))
  (bind _wallthickness (Variables|Settings|Wall|GetWallThickness))
  (bind _wallthickness_2 (Variables|Settings|Wall|GetWallThickness))
  (bind _wallwidth (Variables|Settings|Wall|GetWallWidth))
  (bind _returnvalue (+ _wallthickness_2 _trimthickness))
  (bind _returnvalue_2 (/ _wallwidth 2.0))
  (if (Variables|Settings|Trim|GetbVertical)
    (bind _returnvalue_3 (DynamicMeshActor|AllocateComputeMesh))
    (bind _returnvalue_4 (Class|GeometryScriptLibraryMeshPrimitiveFunctions|AppendRevolvePolygon :TargetMesh _returnvalue_3 :Transform (Math|Transform|MakeTransform (Math|Vector|MakeVector (Utilities|Select :Index Type :NewEnumerator0 _returnvalue_2 :NewEnumerator1 (+ (* _returnvalue_2 -1.0) (Variables|Settings|Trim|GetTrimHeight)) :NewEnumerator2 0.0) (+ (Variables|Settings|ExtendWalls|GetRadius) (/ (Variables|Settings|Wall|GetWallThickness) 2.0)) (Variables|Settings|Wall|GetWallHeight)) "0,90.000000,90.000000" "1.000000,1.000000,1.000000") :PolygonVertices (Utilities|Array|MakeArray (Math|Vector2D|MakeVector2D 0.0 0.0) (Math|Vector2D|MakeVector2D _returnvalue 0.0) (Math|Vector2D|MakeVector2D _returnvalue _trimheight) (Math|Vector2D|MakeVector2D 0.0 _trimheight)) :RevolveOptions (Utilities|Struct|MakeGeometryScriptRevolveOptions 9e+01 -1.8e+02 false false 3e+01 false true) :Radius (- (Variables|Settings|ExtendWalls|GetRadius) (/ _trimthickness 2.0)) :Steps (Variables|Settings|ExtendWalls|GetSteps) :Debug 0))
    (bind _returnvalue_5 (GeometryScript|Materials|RemapMaterialIDs _returnvalue_4 0 3 0))
    (bind _returnvalue_6 (GeometryScript|Booleans|ApplyMeshBoolean :TargetMesh (Variables|Default|GetDynamicMEsh) :ToolMesh _returnvalue_5 :Operation "Union" :Debug 0))
    (bind _returnvalue_7 (DynamicMeshActor|AllocateComputeMesh))
    (bind _returnvalue_8 (Class|GeometryScriptLibraryMeshPrimitiveFunctions|AppendBox :TargetMesh _returnvalue_7 :DimensionX (Variables|Settings|Trim|GetTrimHeight) :DimensionY (+ (Variables|Settings|Trim|GetTrimThickness) (Variables|Settings|Wall|GetWallThickness)) :DimensionZ (Variables|Settings|ExtendWalls|GetExtensionLenght) :Debug 0))
    (bind _returnvalue_9 (GeometryScript|Materials|RemapMaterialIDs _returnvalue_8 0 3 0))
    (bind _returnvalue_10 (GeometryScript|Booleans|ApplyMeshBoolean :TargetMesh _returnvalue_6 :ToolMesh _returnvalue_9 :ToolTransform (Math|Transform|MakeTransform (Math|Vector|MakeVector (Utilities|Select :Index Type :NewEnumerator0 (|((WallW/2)-(TrimH/2)) (Variables|Settings|Wall|GetWallWidth) (Variables|Settings|Trim|GetTrimHeight)) :NewEnumerator1 (+ (* (/ (Variables|Settings|Wall|GetWallWidth) 2.0) -1.0) (/ (Variables|Settings|Trim|GetTrimHeight) 2.0)) :NewEnumerator2 0.0) (|((WThick/2)+Rad) _radius _wallthickness) (|((WHeith+(WThick/2))+Rad) (Variables|Settings|Wall|GetWallHeight) _wallthickness _radius)) "0, 0,90.000000" "1.000000,1.000000,1.000000") :Operation "Union" :Debug 0))
    (Variables|Default|SetDynamicMEsh _returnvalue_10))
  (return))

(fn FnBevel
  (params (TargetMesh :type Dynamic%20Mesh%20Object%20Reference) (Options%20Bevel%20Distance :type Float%20%28double-precision%29))
  (bind _returnvalue (Class|GeometryScriptLibraryMeshPolygroupFunctions|ComputePolygroupsfromAngleThreshold TargetMesh (Utilities|Struct|MakeGeometryScriptGroupLayer true 0) 25.0 2 0))
  (bind _returnvalue_2 (Class|GeometryScriptLibraryMeshModelingFunctions|ApplyMeshPolygroupBevel _returnvalue (Utilities|Struct|MakeGeometryScriptMeshBevelOptions Options%20Bevel%20Distance true 0 false "(Min=(X=0.000000,Y=0.000000,Z=0.000000),Max=(X=0.000000,Y=0.000000,Z=0.000000),IsValid=0)" "0.000000,0.000000,0.000000|0.000000,0.000000,-0.000000|1.000000,1.000000,1.000000" true) 0))
  (bind _returnvalue_3 (Class|GeometryScriptLibraryMeshNormalsFunctions|ComputeSplitNormals _returnvalue_2 (Utilities|Struct|MakeGeometryScriptSplitNormalsOptions true 25.0 false "(bDefaultLayer=True,ExtendedLayerIndex=0)") (Utilities|Struct|MakeGeometryScriptCalculateNormalsOptions true true) 0))
  (return _returnvalue_3))

(fn ApplyMaterials
  (params (Materials :type Array%20of%20Material%20Interface%20Object%20References))
  (Variables|Settings|Wall|SetMaterialWall (Utilities|Array|Get(acopy) Materials))
  (Variables|Settings|Opening|SetMaterialOpeningBorder (Utilities|Array|Get(acopy) Materials 1))
  (Variables|Settings|Glass|SetMaterialGlass (Utilities|Array|Get(acopy) Materials 2))
  (Variables|Settings|Trim|SetMaterialTrim (Utilities|Array|Get(acopy) Materials 3))
  (return))